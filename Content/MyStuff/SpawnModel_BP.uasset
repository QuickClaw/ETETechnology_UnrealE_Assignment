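; SpawnModel_BP spawns a random furniture actor (Couch, Table or Chair) at each of its TargetPoints when play begins.
; Each spawn picks its class through a random integer Select, uses the point's transform and gets a debug label with its object name.
; It then counts the actors of each class in the world and prints the three totals in different colors.
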(event `self.ReceiveBeginPlay`
  (for _array_element (`self.TargetPoints`)
    (bind _returnvalue (`|SpawnActorFromClass` (select `int` (`KismetMathLibrary.RandomInteger` 3) :`0` (`self.Couch`) :`1` (`self.Table`) :`2` (`self.Chair`)) (`self.GetTransform` _array_element) "Undefined" "OverrideRootScale" null null))
    (`KismetSystemLibrary.DrawDebugString` (0.0 0.0 0.0) (`KismetSystemLibrary.GetObjectName` _returnvalue) _returnvalue (struct :`R` 0.630208 :`B` 0.469217 :`A` 1.0) 60.0))
  (bind _outactors (`GameplayStatics.GetAllActorsOfClass` "/Game/MyStuff/Couch.Couch_C"))
  (bind _outactors_2 (`GameplayStatics.GetAllActorsOfClass` "/Game/MyStuff/Table.Table_C"))
  (bind _outactors_3 (`GameplayStatics.GetAllActorsOfClass` "/Game/MyStuff/Chair.Chair_C"))
  (`KismetSystemLibrary.PrintString` (`KismetStringLibrary.Conv_IntToString` (`KismetArrayLibrary.Array_Length` _outactors)) true true (struct :`G` 0.871367 :`B` 1.0 :`A` 1.0) 60.0)
  (`KismetSystemLibrary.PrintString` (`KismetStringLibrary.Conv_IntToString` (`KismetArrayLibrary.Array_Length` _outactors_2)) true true (struct :`G` 0.709804 :`B` 0.011765 :`A` 1.0) 60.0)
  (`KismetSystemLibrary.PrintString` (`KismetStringLibrary.Conv_IntToString` (`KismetArrayLibrary.Array_Length` _outactors_3)) true true (struct :`R` 0.250158 :`G` 0.078187 :`A` 1.0) 60.0))

(fn `UserConstructionScript`)